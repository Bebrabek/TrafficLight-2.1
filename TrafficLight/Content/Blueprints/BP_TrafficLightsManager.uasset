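; Traffic light manager Blueprint that cycles a set of lights in an endless timed loop starting on BeginPlay.
; Recolor steps through light indices 0, 1, 2, 1, with fixed delays after the first three steps before looping back.
; TrafficLightFun stops the three lights in the LightRed array, then recolors the selected one using its NumLight as the key into the ColorSettings color map.
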(event Custom|Recolor
  (CallFunction|TrafficLightFun :!label _label)
  (Utilities|FlowControl|Delay 5.0)
  (CallFunction|TrafficLightFun 1)
  (Utilities|FlowControl|Delay 2.0)
  (CallFunction|TrafficLightFun 2)
  (Utilities|FlowControl|Delay 3.0)
  (CallFunction|TrafficLightFun 1)
  (goto _label))

(event EventBeginPlay
  (CallFunction|Recolor))

(fn ConstructionScript)

(fn TrafficLightFun
  (params (Index :type Integer))
  (bind _lightred (Variables|Default|GetLightRed))
  (bind _output (Utilities|Array|Get(acopy) _lightred Index))
  (for _index (range 0 2)
    (Default|Stop (Utilities|Array|Get(acopy) (Variables|Default|GetLightRed) _index)))
  (Default|ChangeColor _output (.Value (Utilities|Map|Find (.colormap (Variables|Default|GetColorSettings)) (Variables|/Game/Blueprints/BP_TraffictLight.BP_TraffictLight_C|GetNumLight _output)))))